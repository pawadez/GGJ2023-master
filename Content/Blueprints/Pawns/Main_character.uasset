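; Player character Blueprint handling movement, jumping and pausing.
; The MoveRight axis adds movement along the forward vector of the control rotation's yaw, so it drives a single axis of motion.
; Jump uses LaunchCharacter with a fixed upward velocity that overrides Z, with no grounded check in the graph.
; Pause creates the PauseMenu widget, pauses the game and shows the mouse cursor.
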(event `InputAxis|MoveRight`
  (params (AxisValue :type "Float (single-precision)"))
  ;[1 1 1] Movements
  (`self.AddMovementInput` (`KismetMathLibrary.GetForwardVector` (`KismetMathLibrary.MakeRotator` 0.0 0.0 (.yaw (`self.GetControlRotation`)))) AxisValue))

(event `InputAction|Jump`
  (params (Key :type "Key Structure"))
  ;[1 1 1] Movements
  (:`Pressed`
    (`self.LaunchCharacter` (0.0 0.0 2500.0) false true)))

(event `InputAction|Pause`
  (params (Key :type "Key Structure"))
  ;[1 1 1] Pause
  (:`Pressed`
    (bind _returnvalue (`|CreateWidget` "/Game/UI/PauseMenu.PauseMenu_C"))
    (`UserWidget.AddToPlayerScreen` _returnvalue 1000)
    (`GameplayStatics.SetGamePaused` true)
    (set `PlayerController.bShowMouseCursor` true (`GameplayStatics.GetPlayerController` 0))))

(fn `UserConstructionScript`)